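; AC_Status is a character status component that tracks health and stamina, both filled to maximum on BeginPlay.
; Tick drains stamina while sprinting, regenerates it otherwise, forces sprint off at zero, and prints both values for debugging.
; SwitchToSprint allows sprinting only above 10% stamina and broadcasts state through a delegate.
; MakeDamageHealth subtracts clamped damage and fires OnDeath when health reaches zero.
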(event `self.ReceiveBeginPlay`
  ;[0.126 1 0] Указывает на состояние ХП
  (set `self.currentHP` (`self.MaxHP`))
  ;[1 1 1] CuttentStamina - текущие показатели
  (set `self.CurrentStamina` (`self.MaxStamina`)))

(event `self.ReceiveTick`
  (params (DeltaSeconds :type "Float (single-precision)"))
  (set `self.Delta Seconds` DeltaSeconds)
  ;[0.126 1 0] Показывает состояние о ХП
  (`KismetSystemLibrary.PrintString` (`KismetStringLibrary.Conv_DoubleToString` (`self.currentHP`)) true true (struct :`G` 1.0 :`B` 0.361831 :`A` 1.0) 0.0)
  (if (`self.ONSprint`)
    ;[1 1 1] Если в спринте, от убавлять
    (set `self.CurrentStamina` (`KismetMathLibrary.FClamp` (- (`self.CurrentStamina`) (* (`self.StaminaDecrasePerSec`) (`self.Delta Seconds`))) 0.0 (`self.MaxStamina`)))
    (else
      ;[1 1 1] Если  НЕспринте, то прибавлять
      (set `self.CurrentStamina` (`KismetMathLibrary.FClamp` (+ (`self.CurrentStamina`) (* (`self.Delta Seconds`) (`self.StaminaRegenPerSec`))) 0.0 (`self.MaxStamina`)))))
  ;[1 1 1] Если значения спринта становится <=0
  (if (<= (`self.CurrentStamina`) 0.0)
    (`self.SwitchToSprint` false))
  ;[1 1 1] Отображение значений
  (`KismetSystemLibrary.PrintString` (`KismetStringLibrary.Conv_DoubleToString` (`self.CurrentStamina`)) true true (struct :`G` 0.66 :`B` 1.0 :`A` 1.0) 0.0))

(fn `makeDamage/Health`
  (params (Value :type "Float (double-precision)"))
  ;[1 1 1] Value - сделали входящий урон
  (set `self.currentHP` (`KismetMathLibrary.FClamp` (- (`self.currentHP`) Value) 0.0 (`self.MaxHP`)))
  ;[1 1 1] Если значение здоровья <=0, то выскакивает оповещение
  (if (<= (`self.currentHP`) 0.0)
    (`self.OnDeath`)))

(fn `SwitchToSprint`
  (params (ONSprint :type Boolean))
  (if ONSprint
    (if (> (`self.CurrentStamina`) (* (`self.MaxStamina`) 0.1))
      ;[1 1 1] Вкл спринт
      (set `self.ONSprint` true)
      ;[1 1 1 1 12] Это ДЕЛЕГАТ. Он Сигналит, что перекл. в режим спринта
      (`self.ONSrprintDelegate` true))
    (else
      ;[1 1 1] Откл спринт
      (set `self.ONSprint` false)
      (`self.ONSrprintDelegate` false))))